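; Puzzle module Blueprint with two mouse-draggable wheels that drive linked gears and sliders and award an inventory item.
; Drag events select a wheel by component tag and accumulate wrap-corrected Atan2 angle deltas.
; ApplyMechanismRotation turns the wheel, drives clamped gears and four sliders, and grants the item once near full slider travel.
; It also plays drag audio, exposes a camera spline, and retains disconnected hover-prompt and solve logic.
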(event `self.ReceiveBeginPlay`
  (set `self.SliderA1StartLoc` (`SceneComponent.RelativeLocation` (`self.SliderMesh_A1`)))
  (set `self.SliderA2StartLoc` (`SceneComponent.RelativeLocation` (`self.SliderMesh_A2`)))
  (set `self.SliderB1StartLoc` (`SceneComponent.RelativeLocation` (`self.SliderMesh_B1`)))
  (set `self.SliderB2StartLoc` (`SceneComponent.RelativeLocation` (`self.SliderMesh_B2`)))
  (set `self.StartGearARotation` (`SceneComponent.RelativeRotation` (`self.GearPivotA`)))
  (set `self.StartGearBRotation` (`SceneComponent.RelativeRotation` (`self.GearPivotB`))))

(event `StartWheelDrag`
  (params (MouseWorldLocation :type "Vector Structure") (ClickedWheelPivot :type "SceneComponent Object Reference"))
  ; StartWheelDrag 开始拖拽
  (set `self.ActiveWheelPivot` ClickedWheelPivot)
  (if (== ClickedWheelPivot (`self.WheelAPivot`))
    (set `self.ActiveWheelAngle` (`self.WheelAAngle`))
    (if (not (`self.bSolved`)) :!label _label
      (set `self.bDraggingWheel` true)
      (`|ExecutionSequence`
        (:`then_0`
          (`self.PlayWheelVoiceover`))
        (:`then_1`
          (`self.PlayWheelLoopSound`)))
      (set `self.LastMouseAngle` (`KismetMathLibrary.RadiansToDegrees` (`KismetMathLibrary.Atan2` (.z (- MouseWorldLocation (`SceneComponent.K2_GetComponentLocation` (`self.ActiveWheelPivot`)))) (.x (- MouseWorldLocation (`SceneComponent.K2_GetComponentLocation` (`self.ActiveWheelPivot`))))))))
    (elif (== ClickedWheelPivot (`self.WheelBPivot`))
      (set `self.ActiveWheelAngle` (`self.WheelBAngle`))
      (goto _label))))

(event `UpdateWheelDrag`
  (params (MouseWorldLocation :type "Vector Structure"))
  ; UpdateWheelDrag 拖拽过程中持续旋转
  (if (`self.bDraggingWheel`)
    (bind _output_get (set `self.CurrentMouseAngle` (`KismetMathLibrary.RadiansToDegrees` (`KismetMathLibrary.Atan2` (.z (- MouseWorldLocation (`SceneComponent.K2_GetComponentLocation` (`self.ActiveWheelPivot`)))) (.x (- MouseWorldLocation (`SceneComponent.K2_GetComponentLocation` (`self.ActiveWheelPivot`))))))))
    (bind _output_get_2 (set `self.RawDelta` (- _output_get (`self.LastMouseAngle`))))
    ;; if RawDelta > 180:
    ;;         CorrectedDelta = RawDelta - 360
    (if (> _output_get_2 180.0)
      (set `self.CorrectedDelta` (- (`self.RawDelta`) 360.0))
      (else
        ;; else if RawDelta < -180:
        ;;         CorrectedDelta = RawDelta + 360
        (if (< _output_get_2 -180.0)
          (set `self.CorrectedDelta` (+ (`self.RawDelta`) 360.0))
          (else
            ;; else:
            ;;         CorrectedDelta = RawDelta
            (set `self.CorrectedDelta` (`self.RawDelta`))))))
    (`self.ApplyCorrectedDelta`)
    (`self.ApplyMechanismRotation` (`self.NewWheelAngle`))
    (if (== (`self.ActiveWheelPivot`) (`self.WheelAPivot`))
      (set `self.WheelAAngle` (`self.NewWheelAngle`))
      (elif (== (`self.ActiveWheelPivot`) (`self.WheelBPivot`))
        (set `self.WheelBAngle` (`self.NewWheelAngle`))))))

(event `ApplyCorrectedDelta`
  ; UpdateWheelDrag 拖拽过程中持续旋转
  ;; ApplyCorrectedDelta
  (bind _output_get (set `self.NewWheelAngle` (+ (`self.ActiveWheelAngle`) (`self.CorrectedDelta`))))
  (set `self.ActiveWheelAngle` _output_get)
  (set `self.LastMouseAngle` (`self.CurrentMouseAngle`)))

(event `StopWheelDrag`
  ; StopWheelDrag 结束拖拽
  (set `self.bDraggingWheel` false)
  (set `self.ActiveWheelPivot` null))

(event `self.SpawnCollision_WheelA.OnBeginCursorOver`
  (params (TouchedComponent :type "PrimitiveComponent Object Reference"))
  ; 鼠标悬停触发WheelA Interaction Prompt: Drag and Rotate. (Old System)
)

(event `self.SpawnCollision_WheelA.OnEndCursorOver`
  (params (TouchedComponent :type "PrimitiveComponent Object Reference"))
  ; 鼠标悬停触发WheelA Interaction Prompt: Drag and Rotate. (Old System)
)

(event `self.SpawnCollision_WheelB.OnBeginCursorOver`
  (params (TouchedComponent :type "PrimitiveComponent Object Reference"))
  ; 鼠标悬停触发WheelB Interaction Prompt: Drag and Rotate.(Old System)
)

(event `self.SpawnCollision_WheelB.OnEndCursorOver`
  (params (TouchedComponent :type "PrimitiveComponent Object Reference"))
  ; 鼠标悬停触发WheelB Interaction Prompt: Drag and Rotate.(Old System)
)

(event `/Game/TopDown/Blueprints/Interface/BPI_ModuleInteractable.StartDrag`
  (params (HitComponent :type "PrimitiveComponent Object Reference") (HitLocation :type "Vector Structure"))
  ; Interface事件
  (if (`ActorComponent.ComponentHasTag` HitComponent "WheelA")
    (set `self.ActiveWheel` (`self.WheelMesh_A`))
    (`self.StartWheelDrag` HitLocation (`self.WheelAPivot`))
    (elif (`ActorComponent.ComponentHasTag` HitComponent "WheelB")
      (set `self.ActiveWheel` (`self.WheelMesh_B`))
      (`self.StartWheelDrag` HitLocation (`self.WheelBPivot`)))))

(event `/Game/TopDown/Blueprints/Interface/BPI_ModuleInteractable.UpdateDrag`
  (params (CursorWorldLocation :type "Vector Structure"))
  ; Interface事件
  (`self.UpdateWheelDrag` CursorWorldLocation))

(event `/Game/TopDown/Blueprints/Interface/BPI_ModuleInteractable.EndDrag`
  ; Interface事件
  (`self.StopWheelDrag`))

(event `GrantItem_Event`
  ; 获得物品并添加进背包
  ; Obtain Items and add to Inventory
  (bind _asbp_game_instance (cast `/Game/TopDown/Blueprints/BP_GameInstance` (`GameplayStatics.GetGameInstance`)))
  ;; Add Granted Item into Inventory Items
  (`KismetArrayLibrary.Array_Add` (`/Game/TopDown/Blueprints/BP_GameInstance.InventoryItems` _asbp_game_instance) (`self.GrantedItem`))
  ;; Create ItemPopup Panel
  (bind _returnvalue (`|CreateWidget` "/Game/TopDown/Blueprints/WidgetBlueprint/WBP_ItemPopup.WBP_ItemPopup_C" (`GameplayStatics.GetPlayerController` 0)))
  (set `self.ItemPopupRef` _returnvalue)
  (`UserWidget.AddToViewport` (`self.ItemPopupRef`) 0)
  (bind _asbp_no_character_player_controller (cast `/Game/TopDown/Blueprints/BP_NoCharacterPlayerController` (`GameplayStatics.GetPlayerController` 0)))
  ;; 给Popup窗口添加内容
  ;; Add content to ItemPopup Panel
  (`/Game/TopDown/Blueprints/WidgetBlueprint/WBP_ItemPopup.InitItem` (`self.ItemPopupRef`) (`self.GrantedItem`)))

(fn `AlignSplineStartToPreviewCamera`
  (locals (`300` :type "Float (double-precision)" :default 300.0))
  (bind _cameraspline (`self.CameraSpline`))
  (`SplineComponent.SetLocationAtSplinePoint` (`self.CameraSpline`) 0 (`SceneComponent.K2_GetComponentLocation` (`self.PreviewCamera`)) "World" true)
  (`SplineComponent.SetTangentAtSplinePoint` _cameraspline 0 (* (`SceneComponent.GetForwardVector` (`self.CameraSpline`)) (`local.300`)) "World" true)
  (`SplineComponent.UpdateSpline` _cameraspline))

(fn `ApplyMechanismProgress`
  (params (Progress :type "Float (double-precision)"))
  (bind _returnvalue (* Progress (`self.MaxWheelAngle`)))
  (`SceneComponent.K2_SetRelativeRotation` (`self.WheelAPivot`) (`KismetMathLibrary.MakeRotator` 0.0 _returnvalue) false false)
  (`SceneComponent.K2_SetRelativeRotation` (`self.GearPivotA`) (`KismetMathLibrary.MakeRotator` (* _returnvalue (`self.GearARotationMultiplier`))) false false)
  (`SceneComponent.K2_SetRelativeRotation` (`self.GearPivotB`) (`KismetMathLibrary.MakeRotator` 0.0 (* _returnvalue (`self.GearBRotationMultiplier`))) false false)
  (`SceneComponent.K2_SetRelativeLocation` (`self.SliderMesh_A1`) (+ (`self.SliderA1StartLoc`) (* Progress (* (`self.SliderMoveAxis`) (`self.SliderMoveDistance`)))) false false))

(fn `ApplyMechanismRotation`
  (params (WheelAngle :type "Float (double-precision)"))
  (bind _returnvalue (`KismetMathLibrary.FClamp` (* WheelAngle (`self.SliderMoveDistance`)) 0.0 4700.0))
  (bind _returnvalue_2 (* (`self.SliderMoveAxis`) _returnvalue))
  (if (== (`self.ActiveWheelPivot`) (`self.WheelAPivot`))
    (`SceneComponent.K2_SetRelativeRotation` (`self.WheelAPivot`) (`KismetMathLibrary.MakeRotator` 0.0 (`self.WheelAAngle`)) false false)
    (`SceneComponent.K2_SetRelativeRotation` (`self.GearPivotA`) (`KismetMathLibrary.ComposeRotators` (`KismetMathLibrary.MakeRotator` (`KismetMathLibrary.FClamp` (* WheelAngle (`self.GearARotationMultiplier`)) -180.0 180.0)) (`self.StartGearARotation`)) false false :!label _label)
    (`SceneComponent.K2_SetRelativeRotation` (`self.GearPivotB`) (`KismetMathLibrary.ComposeRotators` (`KismetMathLibrary.MakeRotator` 0.0 (`KismetMathLibrary.FClamp` (* WheelAngle (`self.GearBRotationMultiplier`)) -180.0 180.0)) (`self.StartGearBRotation`)) false false)
    (`SceneComponent.K2_SetRelativeLocation` (`self.SliderMesh_A1`) (+ (`self.SliderA1StartLoc`) _returnvalue_2) false false)
    (`SceneComponent.K2_SetRelativeLocation` (`self.SliderMesh_A2`) (+ (`self.SliderA2StartLoc`) _returnvalue_2) false false)
    (`SceneComponent.K2_SetRelativeLocation` (`self.SliderMesh_B1`) (+ (`self.SliderB1StartLoc`) _returnvalue_2) false false)
    (`SceneComponent.K2_SetRelativeLocation` (`self.SliderMesh_B2`) (+ (`self.SliderB2StartLoc`) _returnvalue_2) false false)
    ; GrantItem
    (if (>= _returnvalue 4600.0)
      (if (not (`self.bWheelItemGranted`))
        (`self.GrantItem_Event`)
        (set `self.bWheelItemGranted` true)))
    (elif (== (`self.ActiveWheelPivot`) (`self.WheelBPivot`))
      (`SceneComponent.K2_SetRelativeRotation` (`self.WheelBPivot`) (`KismetMathLibrary.MakeRotator` (`self.WheelBAngle`)) false false)
      (goto _label))))

(fn `GetCameraSpline`
  (returns (CameraSpline :type "SplineComponent Object Reference") (CameraMoveSpeed :type "Float (double-precision)"))
  (return (`self.CameraSpline`) (`self.CameraMoveSpeed`)))

(fn `PlayWheelLoopSound`
  (`/Engine/EditorBlueprintResources/StandardMacros.IsValid` (`self.WheelAudioComponent`)
    (:`Is Not Valid`
      (bind _returnvalue (`GameplayStatics.SpawnSoundAttached` (`self.WheelLoopSound`) (`self.ActiveWheelPivot`) "None" (0.0 0.0 0.0) (struct) "KeepRelativeOffset" false 1.0 1.0 0.0 null null false))
      (set `self.WheelAudioComponent` _returnvalue))))

(fn `PlayWheelVoiceover`
  (`/Engine/EditorBlueprintResources/StandardMacros.IsValid` (`self.WheelStartVoiceover`)
    (:`Is Valid`
      (if (not (`self.bHasPlayedStartVoice`))
        (`GameplayStatics.PlaySoundAtLocation` (`self.WheelStartVoiceover`) (`SceneComponent.K2_GetComponentLocation` (`self.ActiveWheelPivot`)) (struct) 1.0 1.0 0.0 null null null null)
        (set `self.bHasPlayedStartVoice` true)))))

(fn `UserConstructionScript`
  ; 设置PreviewCamera 在 Spline 起点
  (`SceneComponent.K2_SetWorldLocationAndRotation` (`self.PreviewCamera`) (.location (`SplineComponent.GetTransformAtDistanceAlongSpline` (`self.CameraSpline`) (`self.PreviewDistance`) "World" false)) (.rotation (`SplineComponent.GetTransformAtDistanceAlongSpline` (`self.CameraSpline`) (`self.PreviewDistance`) "World" false)) false false))