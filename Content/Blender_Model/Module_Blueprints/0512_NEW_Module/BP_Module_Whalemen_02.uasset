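; Whalemen module actor that offers two draggable zoom items, a submarine and a dining area, and can be revealed or hidden as a group.
; Drag interface events route to two zoom-drag components, with component tags choosing which starts.
; BeginPlay binds their click and drag components, claims interaction points by group tag, then hides everything.
; It exposes a camera spline and speed; GetAlreadyRevealed always returns false despite its setter.
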(event `/Game/TopDown/Blueprints/Interface/BPI_ModuleInteractable.StartDrag`
  (params (HitComponent :type "PrimitiveComponent Object Reference") (HitLocation :type "Vector Structure"))
  ; Interface事件
  ;; DragItem分支
  (`|ExecutionSequence`
    (:`then_0`
      (if (`ActorComponent.ComponentHasTag` HitComponent "DragItemA")
        (`/Game/TopDown/Blueprints/BPAC_ZoomDragItem.TryStartZoomDrag` (`self.BPAC_ZoomDragItem_A`) HitComponent HitLocation)))
    (:`then_1`
      (if (`ActorComponent.ComponentHasTag` HitComponent "DragItemB")
        (`/Game/TopDown/Blueprints/BPAC_ZoomDragItem.TryStartZoomDrag` (`self.BPAC_ZoomDragItem_B`) HitComponent HitLocation)))))

(event `/Game/TopDown/Blueprints/Interface/BPI_ModuleInteractable.UpdateDrag`
  (params (CursorWorldLocation :type "Vector Structure"))
  ; Interface事件
  (`/Game/TopDown/Blueprints/BPAC_ZoomDragItem.UpdateZoomDrag` (`self.BPAC_ZoomDragItem_A`) CursorWorldLocation)
  (`/Game/TopDown/Blueprints/BPAC_ZoomDragItem.UpdateZoomDrag` (`self.BPAC_ZoomDragItem_B`) CursorWorldLocation))

(event `/Game/TopDown/Blueprints/Interface/BPI_ModuleInteractable.EndDrag`
  ; Interface事件
  (`/Game/TopDown/Blueprints/BPAC_ZoomDragItem.StopZoomDrag` (`self.BPAC_ZoomDragItem_A`))
  (`/Game/TopDown/Blueprints/BPAC_ZoomDragItem.StopZoomDrag` (`self.BPAC_ZoomDragItem_B`)))

(event `/Game/TopDown/Blueprints/Interface/BPI_SpawnReveal.HideModuleGroup`
  ; Interface事件
  ;; HideModuleGroup
  (`self.SetActorHiddenInGame` true)
  (`self.SetActorEnableCollision` false)
  (`self.SetActorTickEnabled` false)
  (for _array_element (`self.OwnedInteractionPoints`)
    (`self.SetActorHiddenInGame` _array_element true)
    (`self.SetActorEnableCollision` _array_element false)
    (`self.SetActorTickEnabled` _array_element false)))

(event `self.ReceiveBeginPlay`
  (bind _bpac_zoomdragitem_a (`self.BPAC_ZoomDragItem_A`))
  (bind _bpac_zoomdragitem_b (`self.BPAC_ZoomDragItem_B`))
  ; 设置BPAC_ZoomDragItem
  (set `/Game/TopDown/Blueprints/BPAC_ZoomDragItem.ClickableComponent` (`self.SubmarineClickBox`) _bpac_zoomdragitem_a)
  (set `/Game/TopDown/Blueprints/BPAC_ZoomDragItem.DraggableComponent` (`self.SubmarinePivot_DragA`) _bpac_zoomdragitem_a)
  (set `/Game/TopDown/Blueprints/BPAC_ZoomDragItem.ClickableComponent` (`self.DinningAreaClickBox`) _bpac_zoomdragitem_b)
  (set `/Game/TopDown/Blueprints/BPAC_ZoomDragItem.DraggableComponent` (`self.DinningAreaPivot_DragB`) _bpac_zoomdragitem_b)
  (bind _outactors (`GameplayStatics.GetAllActorsWithTag` (`self.ModuleGroupTag`)))
  (for _array_element _outactors
    (bind _asbp_interaction_point (cast `/Game/TopDown/Blueprints/BP_InteractionPoint` _array_element))
    (`KismetArrayLibrary.Array_Add` (`self.OwnedInteractionPoints`) _asbp_interaction_point)
    (set `/Game/TopDown/Blueprints/BP_InteractionPoint.OwningModuleRef` self _asbp_interaction_point))
  (`self.HideModuleGroup`))

(event `/Game/TopDown/Blueprints/Interface/BPI_SpawnReveal.RevealModuleGroup`
  ; Interface事件
  ;; RevealModuleGroup
  (`self.SetActorHiddenInGame` false)
  (`self.SetActorEnableCollision` true)
  (`self.SetActorTickEnabled` true)
  (for _array_element (`self.OwnedInteractionPoints`)
    (`self.SetActorHiddenInGame` _array_element false)
    (`self.SetActorEnableCollision` _array_element true)
    (`self.SetActorTickEnabled` _array_element true)
    (set `/Game/TopDown/Blueprints/BP_InteractionPoint.OwningModuleRef` self _array_element)))

(event `/Game/TopDown/Blueprints/Interface/BPI_SpawnReveal.SetAlreadyRevealed`
  (params (NewValue :type Boolean))
  ; Interface事件
  (set `self.bAlreadyRevealed` NewValue))

(fn `GetAlreadyRevealed`
  (returns (AlreadyRevealed :type Boolean))
  (return false))

(fn `GetCameraSpline`
  (returns (CameraSpline :type "SplineComponent Object Reference") (CameraMoveSpeed :type "Float (double-precision)"))
  (return (`self.CameraSpline`) (`self.CameraMoveSpeed`)))

(fn `UserConstructionScript`)