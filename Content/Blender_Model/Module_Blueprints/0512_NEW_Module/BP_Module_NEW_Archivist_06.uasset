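; BP_Module_NEW_Archivist_06 is a module actor that hides and reveals itself together with its interaction points.
; On BeginPlay it gathers BP_InteractionPoint actors by ModuleGroupTag, sets itself as their owner and hides the group.
; Interface events toggle visibility, collision and tick for the module and points.
; It exposes a camera spline and speed; GetAlreadyRevealed always returns false, ignoring the value SetAlreadyRevealed stores.
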(event `self.ReceiveBeginPlay`
  (bind _outactors (`GameplayStatics.GetAllActorsWithTag` (`self.ModuleGroupTag`)))
  (for _array_element _outactors
    (bind _asbp_interaction_point (cast `/Game/TopDown/Blueprints/BP_InteractionPoint` _array_element))
    (`KismetArrayLibrary.Array_Add` (`self.OwnedInteractionPoints`) _asbp_interaction_point)
    (set `/Game/TopDown/Blueprints/BP_InteractionPoint.OwningModuleRef` self _asbp_interaction_point))
  (`self.HideModuleGroup`))

(event `/Game/TopDown/Blueprints/Interface/BPI_SpawnReveal.HideModuleGroup`
  ; Interface事件
  ;; HideModuleGroup
  (`self.SetActorHiddenInGame` true)
  (`self.SetActorEnableCollision` false)
  (`self.SetActorTickEnabled` false)
  (for _array_element (`self.OwnedInteractionPoints`)
    (`self.SetActorHiddenInGame` _array_element true)
    (`self.SetActorEnableCollision` _array_element false)
    (`self.SetActorTickEnabled` _array_element false)))

(event `/Game/TopDown/Blueprints/Interface/BPI_SpawnReveal.RevealModuleGroup`
  ; Interface事件
  ;; RevealModuleGroup
  (`self.SetActorHiddenInGame` false)
  (`self.SetActorEnableCollision` true)
  (`self.SetActorTickEnabled` true)
  (for _array_element (`self.OwnedInteractionPoints`)
    (`self.SetActorHiddenInGame` _array_element false)
    (`self.SetActorEnableCollision` _array_element true)
    (`self.SetActorTickEnabled` _array_element true)
    (set `/Game/TopDown/Blueprints/BP_InteractionPoint.OwningModuleRef` self _array_element)))

(event `/Game/TopDown/Blueprints/Interface/BPI_SpawnReveal.SetAlreadyRevealed`
  (params (NewValue :type Boolean))
  ; Interface事件
  (set `self.bAlreadyRevealed` NewValue))

(fn `GetAlreadyRevealed`
  (returns (AlreadyRevealed :type Boolean))
  (return false))

(fn `GetCameraSpline`
  (returns (CameraSpline :type "SplineComponent Object Reference") (CameraMoveSpeed :type "Float (double-precision)"))
  (return (`self.CameraSpline`) (`self.CameraMoveSpeed`)))

(fn `UserConstructionScript`)