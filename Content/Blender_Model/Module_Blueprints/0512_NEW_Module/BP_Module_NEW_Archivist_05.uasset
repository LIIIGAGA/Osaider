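; BP_Module_NEW_Archivist_05 is an Archivist module actor with a draggable item and its own camera spline.
; On BeginPlay it hands the item's click box and pivot to a BPACZoomDragItem component.
; Drag interface events forward to that component, which starts a zoom drag only for hits tagged "DragItem", then updates and stops it.
; GetCameraSpline exposes the spline and camera move speed to callers.
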(event `self.ReceiveBeginPlay`
  (bind _bpac_zoomdragitem (`self.BPAC_ZoomDragItem`))
  (set `/Game/TopDown/Blueprints/BPAC_ZoomDragItem.ClickableComponent` (`self.DragItemClicBox`) _bpac_zoomdragitem)
  (set `/Game/TopDown/Blueprints/BPAC_ZoomDragItem.DraggableComponent` (`self.DragItemPivot`) _bpac_zoomdragitem))

(event `/Game/TopDown/Blueprints/Interface/BPI_ModuleInteractable.StartDrag`
  (params (HitComponent :type "PrimitiveComponent Object Reference") (HitLocation :type "Vector Structure"))
  ; Interface事件
  ;; DragItem分支
  (if (`ActorComponent.ComponentHasTag` HitComponent "DragItem")
    (`/Game/TopDown/Blueprints/BPAC_ZoomDragItem.TryStartZoomDrag` (`self.BPAC_ZoomDragItem`) HitComponent HitLocation)))

(event `/Game/TopDown/Blueprints/Interface/BPI_ModuleInteractable.UpdateDrag`
  (params (CursorWorldLocation :type "Vector Structure"))
  ; Interface事件
  (`/Game/TopDown/Blueprints/BPAC_ZoomDragItem.UpdateZoomDrag` (`self.BPAC_ZoomDragItem`) CursorWorldLocation))

(event `/Game/TopDown/Blueprints/Interface/BPI_ModuleInteractable.EndDrag`
  ; Interface事件
  (`/Game/TopDown/Blueprints/BPAC_ZoomDragItem.StopZoomDrag` (`self.BPAC_ZoomDragItem`)))

(fn `GetCameraSpline`
  (returns (CameraSpline :type "SplineComponent Object Reference") (CameraMoveSpeed :type "Float (double-precision)"))
  (return (`self.CameraSpline`) (`self.CameraMoveSpeed`)))

(fn `UserConstructionScript`)