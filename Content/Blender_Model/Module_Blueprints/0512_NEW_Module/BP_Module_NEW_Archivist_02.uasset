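; Archivist puzzle module where dragging a wheel slides a base piece, alongside a zoom-and-drag item on a locker.
; Tagged drag hits route to either wheel rotation, with voiceover and loop sound, or the BPACZoomDragItem component.
; Wrap-corrected Atan2 cursor angles accumulate into wheel pitch, whose clamped fraction of the maximum angle offsets Base1 along X.
; A delayed reset event eases Base1 back home through VInterpTo on Tick after item grant.
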(event `self.ReceiveTick`
  (params (DeltaSeconds :type "Float (single-precision)"))
  (if (`self.bResettingBase1`)
    (`SceneComponent.K2_SetRelativeLocation` (`self.Base_1`) (`KismetMathLibrary.VInterpTo` (`SceneComponent.RelativeLocation` (`self.Base_1`)) (`self.Base1ResetTargetLocation`) DeltaSeconds (`self.Base1ResetSpeed`)) false false)))

(event `self.ReceiveBeginPlay`
  (bind _bpac_zoomdragitem (`self.BPAC_ZoomDragItem`))
  (set `/Game/TopDown/Blueprints/BPAC_ZoomDragItem.ClickableComponent` (`self.LockerClickSphere`) _bpac_zoomdragitem)
  (set `/Game/TopDown/Blueprints/BPAC_ZoomDragItem.DraggableComponent` (`self.LockerPivot`) _bpac_zoomdragitem)
  (add `/Game/TopDown/Blueprints/BPAC_ZoomDragItem.OnItemGranted` (`self.BPAC_ZoomDragItem`) (`|CreateDelegate` :!event `ResetAfterItemGranted`)))

(event `ResetAfterItemGranted`
  ; ResetAfterItemGranted
  (`KismetSystemLibrary.Delay` 1.5)
  (set `self.Base1ResetTargetLocation` (`self.Base1_InitialLocation`))
  (set `self.bResettingBase1` true))

(event `/Game/TopDown/Blueprints/Interface/BPI_ModuleInteractable.StartDrag`
  (params (HitComponent :type "PrimitiveComponent Object Reference") (HitLocation :type "Vector Structure"))
  ; Interface事件
  (`|ExecutionSequence`
    (:`then_0`
      ;; Wheel分支
      (if (`ActorComponent.ComponentHasTag` HitComponent "WheelA")
        (set `self.ActiveWheel` (`self.WheelMesh_A`))
        (`self.StartWheelDrag` HitLocation (`self.WheelAPivot`))))
    (:`then_1`
      ;; DragItem分支
      (if (`ActorComponent.ComponentHasTag` HitComponent "DragItem")
        (`/Game/TopDown/Blueprints/BPAC_ZoomDragItem.TryStartZoomDrag` (`self.BPAC_ZoomDragItem`) HitComponent HitLocation)))))

(event `StartWheelDrag`
  (params (MouseWorldLocation :type "Vector Structure") (ClickedWheelPivot :type "SceneComponent Object Reference"))
  ; StartWheelDrag 开始拖拽
  (set `self.ActiveWheelPivot` ClickedWheelPivot)
  (if (== ClickedWheelPivot (`self.WheelAPivot`))
    (set `self.ActiveWheelAngle` (`self.Wheel AAngle`))
    (if (not (`self.bSolved`))
      (set `self.bDraggingWheel` true)
      (`|ExecutionSequence`
        (:`then_0`
          (`self.PlayWheelVoiceover`))
        (:`then_1`
          (`self.PlayWheelLoopSound`)))
      (set `self.LastMouseAngle` (`KismetMathLibrary.RadiansToDegrees` (`KismetMathLibrary.Atan2` (.z (- MouseWorldLocation (`SceneComponent.K2_GetComponentLocation` (`self.ActiveWheelPivot`)))) (.x (- MouseWorldLocation (`SceneComponent.K2_GetComponentLocation` (`self.ActiveWheelPivot`))))))))))

(event `/Game/TopDown/Blueprints/Interface/BPI_ModuleInteractable.UpdateDrag`
  (params (CursorWorldLocation :type "Vector Structure"))
  ; Interface事件
  (`self.UpdateWheelDrag` CursorWorldLocation)
  (`/Game/TopDown/Blueprints/BPAC_ZoomDragItem.UpdateZoomDrag` (`self.BPAC_ZoomDragItem`) CursorWorldLocation))

(event `UpdateWheelDrag`
  (params (MouseWorldLocation :type "Vector Structure"))
  ; UpdateWheelDrag 拖拽过程中持续旋转
  (if (`self.bDraggingWheel`)
    (bind _output_get (set `self.CurrentMouseAngle` (`KismetMathLibrary.RadiansToDegrees` (`KismetMathLibrary.Atan2` (.z (- MouseWorldLocation (`SceneComponent.K2_GetComponentLocation` (`self.ActiveWheelPivot`)))) (.x (- MouseWorldLocation (`SceneComponent.K2_GetComponentLocation` (`self.ActiveWheelPivot`))))))))
    (bind _output_get_2 (set `self.RawDelta` (- _output_get (`self.LastMouseAngle`))))
    ;; if RawDelta > 180:
    ;;         CorrectedDelta = RawDelta - 360
    (if (> _output_get_2 180.0)
      (set `self.CorrectedDelta` (- (`self.RawDelta`) 360.0))
      (else
        ;; else if RawDelta < -180:
        ;;         CorrectedDelta = RawDelta + 360
        (if (< _output_get_2 -180.0)
          (set `self.CorrectedDelta` (+ (`self.RawDelta`) 360.0))
          (else
            ;; else:
            ;;         CorrectedDelta = RawDelta
            (set `self.CorrectedDelta` (`self.RawDelta`))))))
    (`self.ApplyCorrectedDelta`)
    (`self.ApplyMechanismRotation` (`self.NewWheelAngle`))
    (if (== (`self.ActiveWheelPivot`) (`self.WheelAPivot`))
      (set `self.Wheel AAngle` (`self.NewWheelAngle`)))))

(event `/Game/TopDown/Blueprints/Interface/BPI_ModuleInteractable.EndDrag`
  ; Interface事件
  (`self.StopWheelDrag`)
  (`/Game/TopDown/Blueprints/BPAC_ZoomDragItem.StopZoomDrag` (`self.BPAC_ZoomDragItem`)))

(event `ApplyCorrectedDelta`
  ; UpdateWheelDrag 拖拽过程中持续旋转
  ;; ApplyCorrectedDelta
  (bind _output_get (set `self.NewWheelAngle` (+ (`self.ActiveWheelAngle`) (`self.CorrectedDelta`))))
  (set `self.ActiveWheelAngle` _output_get)
  (set `self.LastMouseAngle` (`self.CurrentMouseAngle`)))

(event `StopWheelDrag`
  ; StopWheelDrag 结束拖拽
  (set `self.bDraggingWheel` false)
  (set `self.ActiveWheelPivot` null))

(event `ResetBase1`
  ; GrantItem之后Reset被移动的组件
  (`SceneComponent.K2_SetRelativeLocation` (`self.Base_1`) (`self.Base1_InitialLocation`) false false))

(fn `ApplyMechanismRotation`
  (params (`Wheel Angle` :type "Float (double-precision)"))
  (`SceneComponent.K2_SetRelativeRotation` (`self.WheelAPivot`) (`KismetMathLibrary.MakeRotator` 0.0 `Wheel Angle`) false false)
  (`self.UpdateBaseByWheel` (`KismetMathLibrary.FClamp` (/ `Wheel Angle` (`self.MaxWheelAngle`)))))

(fn `GetCameraSpline`
  (returns (CameraSpline :type "SplineComponent Object Reference") (CameraMoveSpeed :type "Float (double-precision)"))
  (return (`self.CameraSpline`) (`self.CameraMoveSpeed`)))

(fn `PlayWheelLoopSound`
  (`/Engine/EditorBlueprintResources/StandardMacros.IsValid` (`self.WheelAudioComponent`)
    (:`Is Not Valid`
      (bind _returnvalue (`GameplayStatics.SpawnSoundAttached` (`self.WheelLoopSound`) (`self.ActiveWheelPivot`) "None" (0.0 0.0 0.0) (struct) "KeepRelativeOffset" false 1.0 1.0 0.0 null null false))
      (set `self.WheelAudioComponent` _returnvalue))))

(fn `PlayWheelVoiceover`
  (`/Engine/EditorBlueprintResources/StandardMacros.IsValid` (`self.WheelStartVoiceover`)
    (:`Is Valid`
      (if (not (`self.bHasPlayedStartVoice`))
        (`GameplayStatics.PlaySoundAtLocation` (`self.WheelStartVoiceover`) (`SceneComponent.K2_GetComponentLocation` (`self.ActiveWheelPivot`)) (struct) 1.0 1.0 0.0 null null null null)
        (set `self.bHasPlayedStartVoice` true)))))

(fn `UpdateBaseByWheel`
  (params (InputAlpha :type "Float (double-precision)"))
  (set `self.WheelAlpha` (`KismetMathLibrary.FClamp` InputAlpha))
  (`SceneComponent.K2_SetRelativeLocation` (`self.Base_1`) (`KismetMathLibrary.MakeVector` (- (.x (`self.Base1_InitialLocation`)) (* (`self.Base1_MoveDistance`) (`self.WheelAlpha`))) (.y (`self.Base1_InitialLocation`)) (.z (`self.Base1_InitialLocation`))) false false))

(fn `UserConstructionScript`)